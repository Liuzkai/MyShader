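; Changer actor that drives an animated material effect on a configurable static mesh.
; The construction script assigns the mesh, creates a dynamic material instance on the chosen slot, and passes it the Range plus an Axis vector taken from the rotated Arrow's forward direction.
; Tick advances a phase by Rate and feeds an offset, scaled absolute sine into the RotationArea parameter for a repeating sweep, leaving the visual change to the material.
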(event `self.ReceiveTick`
  (params (DeltaSeconds :type "Float (single-precision)"))
  (set `self.RotationArea` (+ (* DeltaSeconds (`self.rate`)) (`self.RotationArea`)))
  (`MaterialInstanceDynamic.SetScalarParameterValue` (`self.DMI`) "RotationArea" (* (- (`KismetMathLibrary.Abs` (`KismetMathLibrary.Sin` (`self.RotationArea`))) 0.2) 15.0)))

(fn `UserConstructionScript`
  (`SceneComponent.K2_SetRelativeRotation` (`self.Arrow`) (`self.Axis`) false false)
  (`StaticMeshComponent.SetStaticMesh` (`self.StaticMesh`) (`self.TheChangingMesh`))
  (bind _returnvalue (`PrimitiveComponent.CreateDynamicMaterialInstance` (`self.StaticMesh`) (`self.MaterialSlotIndex`) null "None"))
  (set `self.DMI` _returnvalue)
  (`MaterialInstanceDynamic.SetVectorParameterValue` (`self.DMI`) "Axis" (`KismetMathLibrary.Conv_VectorToLinearColor` (`SceneComponent.GetForwardVector` (`self.Arrow`))))
  (`MaterialInstanceDynamic.SetScalarParameterValue` (`self.DMI`) "Range" (`self.Range`)))